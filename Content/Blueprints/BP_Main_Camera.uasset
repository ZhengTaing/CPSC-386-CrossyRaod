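; BP_Main_Camera is the follow camera for a Crossy Road-style game, tracking the player's chicken.
; BeginPlay caches the player pawn as BP_Chicken and hands that reference to BP_GameMode_CrossyRoad.
; Tick moves the actor along the chicken's Y position plus an offset, keeping X and height fixed, with no smoothing.
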(event `self.ReceiveBeginPlay`
  (bind _asbp_chicken (cast `/Game/Blueprints/BP_Chicken` (`GameplayStatics.GetPlayerPawn` 0)))
  (set `self.CHICKEN ref` _asbp_chicken)
  (bind _asbp_game_mode_crossy_road (cast `/Game/Blueprints/BP_GameMode_CrossyRoad` (`GameplayStatics.GetGameMode`)))
  (set `/Game/Blueprints/BP_GameMode_CrossyRoad.Chicken REF` (`self.CHICKEN ref`) _asbp_game_mode_crossy_road))

(event `self.ReceiveTick`
  (params (DeltaSeconds :type "Float (single-precision)"))
  (`self.K2_SetActorLocation` (`KismetMathLibrary.MakeVector` 0.0 (+ (`.Y` (`KismetMathLibrary.BreakVector3f` (`self.K2_GetActorLocation` (`self.CHICKEN ref`)))) (`self.offsetY`)) 1300.0)))

(fn `UserConstructionScript`)