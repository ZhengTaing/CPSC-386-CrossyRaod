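; Vehicle spawner that emits BP_Vehicle actors at one shared random speed, passing each a facing direction and chicken reference.
; Tick spawns a vehicle at the spawner's transform whenever a timer reaches a re-randomized interval of a few seconds.
; BeginPlay also runs an initial spawn loop at an offset position.
; That loop accumulates random distances without applying them to the position and never updates its ContinuewVehicle condition.
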(event `self.ReceiveBeginPlay`
  (set `self.speed` (`KismetMathLibrary.RandomFloatInRange` 300.0 600.0))
  (`self.setNewMax`)
  (`self.spawnInitVechicle`))

(event `self.ReceiveTick`
  (params (DeltaSeconds :type "Float (single-precision)"))
  (bind _output_get (set `self.accumTime` (+ DeltaSeconds (`self.accumTime`))))
  (if (>= _output_get (`self.maxTime`))
    (set `self.accumTime` 0.0)
    (`self.setNewMax`)
    (`|SpawnActorFromClass` "/Game/Blueprints/BP_Vehicle.BP_Vehicle_C" (`self.GetTransform`) "Undefined" "OverrideRootScale" null (`self.facingLeft`) (`self.speed`) (`self.Chicken REF`) null)))

(fn `setNewMax`
  (set `self.maxTime` (`KismetMathLibrary.RandomFloatInRange` 2.0 5.0)))

(fn `spawnInitVechicle`
  (locals (numofVehicle :type Integer) (Xinit :type "Float (double-precision)") (XAccum :type "Float (double-precision)") (distanceAccum :type "Float (double-precision)") (continuewVehicle :type Boolean))
  (bind (_returnvalue_x _returnvalue_y) (`KismetMathLibrary.BreakVector` (`self.K2_GetActorLocation`)))
  (bind _returnvalue (`KismetMathLibrary.RandomFloatInRange` 600.0 1200.0))
  (bind (_returnvalue_x_2 _returnvalue_y_2 _returnvalue_z) (`KismetMathLibrary.BreakVector` (`self.K2_GetActorLocation`)))
  (if (`self.facingLeft`)
    (set `local.Xinit` (+ _returnvalue_x -600.0))
    (else
      (set `local.Xinit` (+ _returnvalue_y 600.0))))
  (while (`local.continuewVehicle`)
    (set `local.XAccum` _returnvalue)
    (set `local.distanceAccum` (+ _returnvalue (`local.distanceAccum`)))
    (if (`self.facingLeft`)
      (set `local.XAccum` (* (`local.XAccum`) -1.0)))
    (`|SpawnActorFromClass` "/Game/Blueprints/BP_Vehicle.BP_Vehicle_C" (`KismetMathLibrary.MakeTransform` (`KismetMathLibrary.MakeVector` (`local.Xinit`) _returnvalue_y_2 _returnvalue_z)) "Undefined" "OverrideRootScale" null (`self.facingLeft`) (`self.speed`) (`self.Chicken REF`) null)))

(fn `UserConstructionScript`)