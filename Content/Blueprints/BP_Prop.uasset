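; BP_Prop is a prop with a static mesh and an optional Dark flag meant to darken its material.
; On BeginPlay it creates and stores a dynamic instance of the chicken colors material, then calls Darken if the flag is set.
; Darken only reads the "darkness" vector parameter.
; The node that would write back a reduced value is never executed, so the prop's appearance is unchanged.
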(event `self.ReceiveBeginPlay`
  (bind _returnvalue (`PrimitiveComponent.CreateDynamicMaterialInstance` (`self.StaticMesh`) 0 "/Game/media/meshes/M_chicken__colors_png.M_chicken__colors_png" "None"))
  (set `self.materialInstance` _returnvalue)
  (if (`self.dark`)
    (`self.darken`)))

(fn `darken`
  (bind _returnvalue (`MaterialInstanceDynamic.K2_GetVectorParameterValue` (`self.materialInstance`) "darkness")))

(fn `UserConstructionScript`)