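; BP_Bounce is an actor that plays a procedural vertical bounce while its JumpedOn flag is true.
; Tick runs BouncingAnim, which advances a timer and sets the actor's height to CachedZpos plus an offset.
; After a start delay, JumpedOnAnim computes that offset from a squared-time parabola over a short window.
; ResetAnim then clears timer and offset but sets JumpedOn true, so the cycle repeats.
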(event `self.ReceiveBeginPlay`
  (set `self.maxJOT` (+ (`self.maxStartJT`) 0.2)))

(event `self.ReceiveTick`
  (params (DeltaSeconds :type "Float (single-precision)"))
  (`self.bouncingAnim` DeltaSeconds))

(fn `bouncingAnim`
  (params (deltaTime :type "Float (double-precision)"))
  (bind (_returnvalue_x _returnvalue_y) (`KismetMathLibrary.BreakVector` (`self.K2_GetActorLocation`)))
  (if (`self.jumpedOn`)
    (`self.jumpedOnAnim` deltaTime)
    (`self.K2_SetActorLocation` (`KismetMathLibrary.MakeVector` _returnvalue_x _returnvalue_y (+ (`self.cachedZpos`) (`self.jumpedOnZ`))))))

(fn `jumpedOnAnim`
  (params (deltaTime :type "Float (double-precision)"))
  (set `self.currJOT` (+ deltaTime (`self.currJOT`)))
  (if (>= (`self.currJOT`) (`self.maxStartJT`))
    (if (>= (`self.currJOT`) (`self.maxJOT`))
      (`self.resetAnim`)
      (else
        (set `self.jumpedOnZ` (* (- (`KismetMathLibrary.Square` (- (* (- (`self.currJOT`) 0.1) 8.0) 1.0)) 1.0) 20.0))))))

(fn `resetAnim`
  (set `self.jumpedOn` true)
  (set `self.jumpedOnZ` 0.0)
  (set `self.currJOT` 0.0))

(fn `UserConstructionScript`)