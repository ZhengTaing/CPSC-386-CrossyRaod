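; BP_Log is a moving log obstacle that drifts along the X axis and can be jumped on.
; On BeginPlay its Length picks one of three meshes and a matching X scale for the box.
; Each tick moves it in its set direction, with separate center and outer-zone speeds plus a random offset, and destroys it past the X limits.
; Tick also triggers a random landing sound and calls a bouncing animation.
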(event `self.ReceiveBeginPlay`
  (bind _staticmesh (`self.StaticMesh`))
  (`parent.ReceiveBeginPlay`)
  (switch `int` (`self.length`)
    (:`1`
      (set `self.scaleX` 1.75)
      (`StaticMeshComponent.SetStaticMesh` _staticmesh "/Game/media/meshes/log3.log3"))
    (:`2`
      (set `self.scaleX` 5.0)
      (`StaticMeshComponent.SetStaticMesh` _staticmesh "/Game/media/meshes/log2.log2"))
    (:`3`
      (set `self.scaleX` 8.5)
      (`StaticMeshComponent.SetStaticMesh` _staticmesh "/Game/media/meshes/log1.log1")))
  (`SceneComponent.SetRelativeScale3D` (`self.Box`) (`KismetMathLibrary.MakeVector` (`self.scaleX`))))

(event `self.ReceiveTick`
  (params (DeltaSeconds :type "Float (single-precision)"))
  (`self.moveLog` DeltaSeconds)
  (`self.logOutofBounds`)
  (`self.jumpedOnSound`)
  (`self.bouncingAnim` DeltaSeconds))

(fn `jumpedOnSound`
  (bind _returnvalue (`KismetMathLibrary.RandomFloatInRange` 0.0))
  (if (and (== (`self.currJOT`) 0.0) (`self.jumpedOn`))
    (if (`KismetMathLibrary.RandomBool`)
      (`GameplayStatics.PlaySound2D` "/Game/media/sounds/log1.log1" _returnvalue 1.0 0.0 null null)
      (else
        (`GameplayStatics.PlaySound2D` "/Game/media/sounds/log2.log2" _returnvalue 1.0 0.0 null null)))))

(fn `logOutofBounds`
  (bind _returnvalue_x (`KismetMathLibrary.BreakVector` (`self.K2_GetActorLocation`)))
  (if (> _returnvalue_x 2800.0)
    (`self.K2_DestroyActor` :!label _label)
    (elif (< _returnvalue_x -2800.0)
      (goto _label))))

(fn `moveLog`
  (params (deltaTime :type "Float (double-precision)"))
  (bind _returnvalue_x (`KismetMathLibrary.BreakVector` (`self.K2_GetActorLocation`)))
  (if (`self.move_left`)
    (set `self.float_inverse` -1.0))
  (if (>= _returnvalue_x -1400.0)
    (if (<= _returnvalue_x 1400.0)
      (set `self.currSpeed` (`self.ms_center`))
      (else
        (set `self.currSpeed` (`self.ms_left_or_right`) :!label _label)))
    (else
      (goto _label)))
  (bind _output_get (set `self.currSpeed` (* (`self.float_inverse`) (+ (`self.currSpeed`) (`self.ms_random`)))))
  (`self.K2_AddActorWorldOffset` (`KismetMathLibrary.MakeVector` (* _output_get deltaTime))))

(fn `UserConstructionScript`
  (`parent.UserConstructionScript`))