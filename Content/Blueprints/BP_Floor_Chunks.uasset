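; BP_Floor_Chunks is a floor row for a chicken game, holding left, center and right floor pieces, landing nodes and props.
; Helpers compute the three floor transforms and give a one-in-ten chance of spawning a coin.
; Every Tick it destroys its pieces and itself once its Y reaches the chicken's plus MaxDistanceBehindChicken.
; The landing-node spawn logic is present but disconnected, so that function does nothing here.
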(event `self.ReceiveTick`
  (params (DeltaSeconds :type "Float (single-precision)"))
  (`self.isFloordestoryed`))

(fn `calcFloortransform`
  (returns (transLeft :type "Transform Structure") (transCenter :type "Transform Structure") (transRight :type "Transform Structure") (yPos :type "Float (double-precision)"))
  (bind _positiony (`self.positionY`))
  (return (`KismetMathLibrary.MakeTransform` (`KismetMathLibrary.MakeVector` -1800.0 _positiony)) (`KismetMathLibrary.MakeTransform` (`KismetMathLibrary.MakeVector` 0.0 _positiony)) (`KismetMathLibrary.MakeTransform` (`KismetMathLibrary.MakeVector` 1800.0 _positiony)) _positiony))

(fn `constructLandingnode (floor chunk)`
  (params (isWater :type Boolean)))

(fn `createCoin`
  (bind (_returnvalue_x _returnvalue_y) (`KismetMathLibrary.BreakVector` (`self.K2_GetActorLocation`)))
  (if (== (`KismetMathLibrary.RandomInteger` 9) 0)
    (`|SpawnActorFromClass` "/Game/Blueprints/BP_Coin.BP_Coin_C" (`KismetMathLibrary.MakeTransform` (`KismetMathLibrary.MakeVector` (`self.currentXpos`) _returnvalue_y (`self.currentZpos`))) "Undefined" "OverrideRootScale" null null)))

(fn `destroyMeshes`
  (for _array_element (`self.landingNodes`)
    (`self.K2_DestroyActor` _array_element))
  (`self.K2_DestroyActor` (`self.leftFloor`))
  (`self.K2_DestroyActor` (`self.rightFloor`))
  (`self.K2_DestroyActor` (`self.centerFloor`))
  (for _array_element_2 (`self.props`)
    (`self.K2_DestroyActor` _array_element_2)))

(fn `isFloordestoryed`
  (bind (_returnvalue_x _returnvalue_y) (`KismetMathLibrary.BreakVector` (`self.K2_GetActorLocation`)))
  (bind _chickenref (`self.chickenRef`))
  (bind (_returnvalue_x_2 _returnvalue_y_2) (`KismetMathLibrary.BreakVector` (`self.K2_GetActorLocation` _chickenref)))
  (if (`KismetSystemLibrary.IsValid` _chickenref)
    (if (>= _returnvalue_y (+ _returnvalue_y_2 (`self.maxDistance_behindChicken`)))
      (`self.destroyMeshes`)
      (`self.K2_DestroyActor`))))

(fn `UserConstructionScript`)