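; BP_Feather is an actor that falls while tumbling, like a drifting feather.
; On BeginPlay it picks a random rotation and caches its spawn location.
; Each Tick it spins all rotation axes at a constant rate and lowers the cached location at a steady speed, setting both directly without sweep or physics.
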(event `self.ReceiveBeginPlay`
  (set `self.rotation` (`KismetMathLibrary.RandomRotator` false))
  (set `self.location` (`self.K2_GetActorLocation`)))

(event `self.ReceiveTick`
  (params (DeltaSeconds :type "Float (single-precision)"))
  (bind _returnvalue (* DeltaSeconds 100.0))
  (bind (_rotation_roll _rotation_pitch _rotation_yaw) (`KismetMathLibrary.BreakRotator` (`self.rotation`)))
  (bind (_location_x _location_y _location_z) (`KismetMathLibrary.BreakVector` (`self.location`)))
  (bind _output_get (set `self.rotation` (`KismetMathLibrary.MakeRotator` (+ _rotation_roll _returnvalue) (+ _rotation_pitch _returnvalue) (+ _rotation_yaw _returnvalue))))
  (`self.K2_SetActorRotation` _output_get)
  (bind _output_get_2 (set `self.location` (`KismetMathLibrary.MakeVector` _location_x _location_y (+ (* DeltaSeconds -100.0) _location_z))))
  (`SceneComponent.K2_SetWorldLocation` (`self.DefaultSceneRoot`) _output_get_2 false false))

(fn `UserConstructionScript`)