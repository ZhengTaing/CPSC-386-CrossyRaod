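; BP_Road is a road floor chunk, apparently for a Crossy Road-style game with a chicken player.
; On BeginPlay it spawns left, traversable center and right floors, plus line props when HasLines is set.
; It adds a vehicle spawner on a random side, facing across the road and given the chicken reference, and destroys it with the chunk.
; A loop creates landing nodes alongside calls to CreateCoin.
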(event `self.ReceiveBeginPlay`
  (bind _props (`self.props`))
  (bind (_transleft _transcenter _transright _ypos) (`self.calcFloortransform`))
  (bind _returnvalue (`|SpawnActorFromClass` "/Game/Blueprints/BP_Floor.BP_Floor_C" _transleft "Undefined" "OverrideRootScale" null 1 false self null))
  (set `self.leftFloor` _returnvalue)
  (bind _returnvalue_2 (`|SpawnActorFromClass` "/Game/Blueprints/BP_Floor.BP_Floor_C" _transcenter "Undefined" "OverrideRootScale" null 1 true self null))
  (set `self.centerFloor` _returnvalue_2)
  (bind _returnvalue_3 (`|SpawnActorFromClass` "/Game/Blueprints/BP_Floor.BP_Floor_C" _transright "Undefined" "OverrideRootScale" null 1 false self null))
  (set `self.rightFloor` _returnvalue_3)
  (if (`self.hasLines`)
    (bind _returnvalue_4 (- _ypos -100.0))
    (bind _returnvalue_5 (`|SpawnActorFromClass` "/Game/Blueprints/BP_Road_Lines.BP_Road_Lines_C" (`KismetMathLibrary.MakeTransform` (`KismetMathLibrary.MakeVector` -2000.0 _returnvalue_4)) "Undefined" "OverrideRootScale" null true null))
    (`KismetArrayLibrary.Array_Add` _props _returnvalue_5)
    (bind _returnvalue_6 (`|SpawnActorFromClass` "/Game/Blueprints/BP_Road_Lines.BP_Road_Lines_C" (`KismetMathLibrary.MakeTransform` (`KismetMathLibrary.MakeVector` 0.0 _returnvalue_4)) "Undefined" "OverrideRootScale" null false null))
    (`KismetArrayLibrary.Array_Add` _props _returnvalue_6)
    (bind _returnvalue_7 (`|SpawnActorFromClass` "/Game/Blueprints/BP_Road_Lines.BP_Road_Lines_C" (`KismetMathLibrary.MakeTransform` (`KismetMathLibrary.MakeVector` 2000.0 _returnvalue_4)) "Undefined" "OverrideRootScale" null true null))
    (`KismetArrayLibrary.Array_Add` _props _returnvalue_7))
  (`self.constructVehicleSpawner` _ypos)
  (`self.constructLandingNodes`))

(event `self.ReceiveDestroyed`
  (for _array_element (`self.vehicleSpawner`)
    (`self.K2_DestroyActor` _array_element)))

(fn `constructLandingNodes`
  (set `self.currentZpos` -30.0)
  (for _ (range 9)
    (`self.createCoin`)
    (`self.constructLandingnode (floor chunk)` false)))

(fn `constructVehicleSpawner`
  (params (posY :type "Float (double-precision)"))
  (locals (posX :type "Float (double-precision)") (facingLeft :type Boolean))
  (bind _output_get (set `local.facingLeft` (`KismetMathLibrary.RandomBool`)))
  (if _output_get
    (set `local.posX` 2800.0)
    (else
      (bind _output_get_2 (set `local.posX` -2800.0))))
  (bind _returnvalue (`|SpawnActorFromClass` "/Game/Blueprints/BP_Vehicle_Spawner.BP_Vehicle_Spawner_C" (`KismetMathLibrary.MakeTransform` (`KismetMathLibrary.MakeVector` _output_get_2 posY -10.0)) "Undefined" "OverrideRootScale" null _output_get (`self.chickenRef`) null))
  (`KismetArrayLibrary.Array_Add` (`self.vehicleSpawner`) _returnvalue))

(fn `UserConstructionScript`
  (`parent.UserConstructionScript`))