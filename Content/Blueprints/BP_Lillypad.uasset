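; Lily pad actor that bounces when jumped on and spins while a chicken stands on it.
; BeginPlay picks a random spin rate and spawns an actor at the pad's location.
; Tick plays a 2D lily pad sound at the start of a jumped-on bounce, runs the bounce animation, and applies the spin scaled by delta time.
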(event `self.ReceiveBeginPlay`
  ;[1 1 1] Comment
  (`parent.ReceiveBeginPlay`)
  (set `self.rotation` (`KismetMathLibrary.MakeRotator` 0.0 0.0 (`KismetMathLibrary.RandomFloatInRange` -20.0 20.0)))
  (switch `int` (`KismetMathLibrary.RandomInteger` 3)
    (:`0`
      _)
    (:`1`
      _))
  (`|SpawnActorFromClass` "/Game/Blueprints/BP_Coin.BP_Coin_C" (`KismetMathLibrary.MakeTransform` (`self.K2_GetActorLocation`)) "Undefined" "OverrideRootScale" null null))

(event `self.ReceiveTick`
  (params (DeltaSeconds :type "Float (single-precision)"))
  ;[1 1 1] Comment
  (set `self.mainDeltaSec` DeltaSeconds)
  (`self.attemptJumpedOnSound`)
  (`self.bouncingAnim` (`self.mainDeltaSec`))
  (if (`self.chickenOnTop`)
    (`self.K2_AddActorLocalRotation` (* (`self.rotation`) (`self.mainDeltaSec`)))))

(fn `attemptJumpedOnSound`
  (if (and (== (`self.currJOT`) 0.0) (`self.jumpedOn`))
    (`GameplayStatics.PlaySound2D` "/Game/media/sounds/lily_pad.lily_pad" 1.0 1.0 0.0 null null)))

(fn `UserConstructionScript`
  (`parent.UserConstructionScript`))