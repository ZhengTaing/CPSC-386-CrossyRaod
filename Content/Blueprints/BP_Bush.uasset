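; BP_Bush is a foliage prop actor that varies its look at random through its Construction Script, with no active gameplay logic.
; A random roll picks one of three quarter-turn rotations, then a second roll swaps the static mesh to one of three tree meshes.
; A zero on the first roll skips both steps, and a zero on the second keeps the existing mesh.
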(fn `UserConstructionScript`
  (bind _staticmesh (`self.StaticMesh`))
  (switch `int` (`KismetMathLibrary.RandomIntegerInRange` 0 3)
    (:`1`
      (`self.K2_SetActorRotation` (struct :`Yaw` 90.0)))
    (:`2`
      (`self.K2_SetActorRotation` (struct :`Yaw` 180.0)))
    (:`3`
      (`self.K2_SetActorRotation` (struct :`Yaw` 270.0))))
  (switch `int` (`KismetMathLibrary.RandomIntegerInRange` 0 3)
    (:`1`
      (`StaticMeshComponent.SetStaticMesh` _staticmesh "/Game/media/meshes/tree1.tree1"))
    (:`2`
      (`StaticMeshComponent.SetStaticMesh` _staticmesh "/Game/media/meshes/tree2.tree2"))
    (:`3`
      (`StaticMeshComponent.SetStaticMesh` _staticmesh "/Game/media/meshes/tree3.tree3"))))