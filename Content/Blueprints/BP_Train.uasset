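; BP_Train is a moving train actor that travels along the world X axis for a limited time.
; If MoveLeft is set, BeginPlay rotates it 180 degrees and Tick moves it toward negative X, otherwise toward positive X.
; Each Tick scales movement by MoveSpeed and delta time, counts down Lifespan, and destroys the actor when it runs out.
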(event `self.ReceiveBeginPlay`
  ;[1 1 1] Comment
  (if (`self.move_left`)
    (`self.K2_SetActorRotation` (struct :`Yaw` 180.0))))

(event `self.ReceiveTick`
  (params (DeltaSeconds :type "Float (single-precision)"))
  (bind _returnvalue (* (`self.move_speed`) DeltaSeconds))
  ;[1 1 1] Comment
  (if (`self.move_left`)
    (`self.K2_AddActorWorldOffset` (`KismetMathLibrary.MakeVector` (* _returnvalue -1.0)))
    (else
      (`self.K2_AddActorWorldOffset` (`KismetMathLibrary.MakeVector` _returnvalue))))
  (bind _output_get (set `self.lifespan` (- (`self.lifespan`) DeltaSeconds)))
  (if (<= _output_get 0.0)
    (`self.K2_DestroyActor`)))

(fn `UserConstructionScript`)