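; BP_Water is a water row floor chunk that spawns three floor sections, landing nodes and optional logs or lily pads for crossing.
; Lily pads spawn at up to three supplied clear-column X positions, skipping duplicates, and are destroyed with the chunk.
; Logs pre-fill the row on BeginPlay, then Tick spawns more from one side on timers scaled by log length and the row's random speed bonus.
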(event `self.ReceiveBeginPlay`
  ;[1 1 1] Comment
  (bind (_transleft _transcenter _transright) (`self.calcFloortransform`))
  (bind _returnvalue (`|SpawnActorFromClass` "/Game/Blueprints/BP_Floor.BP_Floor_C" _transleft "Undefined" "OverrideRootScale" null 2 false self null))
  (set `self.leftFloor` _returnvalue)
  (bind _returnvalue_2 (`|SpawnActorFromClass` "/Game/Blueprints/BP_Floor.BP_Floor_C" _transcenter "Undefined" "OverrideRootScale" null 2 true self null))
  (set `self.centerFloor` _returnvalue_2)
  (bind _returnvalue_3 (`|SpawnActorFromClass` "/Game/Blueprints/BP_Floor.BP_Floor_C" _transright "Undefined" "OverrideRootScale" null 2 false self null))
  (set `self.rightFloor` _returnvalue_3)
  (`self.Construct Landing Nodes`)
  (if (`self.createLog`)
    (`self.constructInitialLog`)))

(event `self.ReceiveTick`
  (params (DeltaSeconds :type "Float (single-precision)"))
  ;[1 1 1] Comment
  (if (`self.createLog`)
    (`self.constructLogAttempt` DeltaSeconds))
  (`self.isFloordestoryed`))

(event `self.ReceiveDestroyed`
  ;[1 1 1] Comment
  (for _array_element (`self.lillyPads`)
    (`self.K2_DestroyActor` _array_element)))

(fn `addRandomSpeedLog`
  (set `self.extraLogSpeedCenter` (`KismetMathLibrary.RandomFloatInRange` 0.0 200.0)))

(fn `Calc Log Creation`
  (returns (randomXPos :type "Float (double-precision)"))
  (`/Engine/EditorBlueprintResources/StandardMacros.IsValid` (`self.currLogCreated`)
    (:`Is Valid`
      (switch `int` (`/Game/Blueprints/BP_Log.length` (`self.currLogCreated`))
        (:`1`
          (return (`KismetMathLibrary.RandomFloatInRange` 400.0 500.0)))
        (:`2`
          (return (`KismetMathLibrary.RandomFloatInRange` 600.0 700.0)))
        (:`3`
          (return (`KismetMathLibrary.RandomFloatInRange` 800.0 900.0)))))
    (:`Is Not Valid`
      (return (`KismetMathLibrary.RandomFloatInRange` 0.0 100.0)))))

(fn `Construct Landing Nodes`
  (set `self.currentZpos` -60.0)
  (for _ (range 9)
    (`self.constructLandingnode (floor chunk)` true))
  (if (`self.createLillypad`)
    (`self.constructLillyPads (Multiple)`)))

(fn `Construct Lilly Pad`
  (params (currX :type "Float (double-precision)"))
  (bind (_returnvalue_x _returnvalue_y _returnvalue_z) (`KismetMathLibrary.BreakVector` (`self.K2_GetActorLocation`)))
  (if (not (== currX -1.0))
    (bind _returnvalue (`|SpawnActorFromClass` "/Game/Blueprints/BP_Lillypad.BP_Lillypad_C" (`KismetMathLibrary.MakeTransform` (`KismetMathLibrary.MakeVector` currX _returnvalue_y (- _returnvalue_z 30.0))) "Undefined" "OverrideRootScale" null null))
    (`KismetArrayLibrary.Array_Add` (`self.lillyPads`) _returnvalue)))

(fn `constructInitialLog`
  (locals (logCreateXPos :type "Float (double-precision)"))
  (if (`self.createLogsleft`)
    (set `local.logCreateXPos` -900.0)
    (while (< (`local.logCreateXPos`) 900.0)
      (bind _randomxpos (`self.Calc Log Creation`))
      (bind _output_get (set `local.logCreateXPos` (+ _randomxpos (`local.logCreateXPos`))))
      (`self.constructLog` _output_get))
    (else
      (set `local.logCreateXPos` 900.0)
      (while (> (`local.logCreateXPos`) -900.0)
        (bind _randomxpos_2 (`self.Calc Log Creation`))
        (bind _output_get_2 (set `local.logCreateXPos` (- (`local.logCreateXPos`) _randomxpos_2)))
        (`self.constructLog` _output_get_2)))))

(fn `constructLillyPads (Multiple)`
  (bind _currclearcolmposx3 (`self.currClearColmPosX3`))
  ;[1 1 1] Construct Multiple Lilly Pads
  (if (>= (`self.numberofLillypad`) 1)
    (`self.Construct Lilly Pad` (`self.currClearColmPosX1`))
    (if (>= (`self.numberofLillypad`) 2)
      (if (not (== (`self.currClearColmPosX1`) (`self.currClearColmPosX2`)))
        (`self.Construct Lilly Pad` (`self.currClearColmPosX2`))
        (if (>= (`self.numberofLillypad`) 3)
          (if (not (or (== (`self.currClearColmPosX2`) _currclearcolmposx3) (== _currclearcolmposx3 (`self.currClearColmPosX1`))))
            (`self.Construct Lilly Pad` (`self.currClearColmPosX3`))))))))

(fn `constructLog`
  (params (locationX :type "Float (double-precision)"))
  (returns (returnLog :type "/Game/Blueprints/BP_Log Object Reference"))
  (bind (_returnvalue_x _returnvalue_y _returnvalue_z) (`KismetMathLibrary.BreakVector` (`self.K2_GetActorLocation`)))
  (bind _returnvalue (`|SpawnActorFromClass` "/Game/Blueprints/BP_Log.BP_Log_C" (`KismetMathLibrary.MakeTransform` (`KismetMathLibrary.MakeVector` locationX _returnvalue_y _returnvalue_z)) "Undefined" "OverrideRootScale" null (`KismetMathLibrary.RandomIntegerInRange` 1 3) (not (`self.createLogsleft`)) (`self.extraLogSpeedCenter`) null))
  (bind _output_get (set `self.currLogCreated` _returnvalue))
  (return _output_get))

(fn `constructLogAttempt`
  (params (deltaTime :type "Float (double-precision)"))
  (bind _returnvalue (/ (`self.extraLogSpeedCenter`) 400.0))
  (bind _output_get (set `self.currCreateLogTime` (+ deltaTime (`self.currCreateLogTime`))))
  (if (>= _output_get (`self.maxCreateLogTime`))
    (if (`self.createLogsleft`)
      (`self.constructLog` -2800.0)
      (else
        (`self.constructLog` 2800.0)))
    (set `self.currCreateLogTime` 0.0)
    (switch `int` (`/Game/Blueprints/BP_Log.length` (`self.currLogCreated`))
      (:`1`
        (set `self.maxCreateLogTime` (- (`KismetMathLibrary.RandomFloatInRange` 1.25 1.5) _returnvalue)))
      (:`2`
        (set `self.maxCreateLogTime` (- (`KismetMathLibrary.RandomFloatInRange` 1.5 1.75) _returnvalue)))
      (:`3`
        (set `self.maxCreateLogTime` (- (`KismetMathLibrary.RandomFloatInRange` 2.0 2.25) _returnvalue))))))

(fn `UserConstructionScript`
  (if (`self.createLog`)
    (set `self.maxCreateLogTime` (`KismetMathLibrary.RandomFloatInRange` 0.0 1.0))
    (`self.addRandomSpeedLog`)))